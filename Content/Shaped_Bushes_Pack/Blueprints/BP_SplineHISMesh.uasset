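; Spline placement actor from the Shaped Bushes pack that distributes instanced meshes evenly along an editable spline.
; The construction script creates one HISM component per mesh array entry, then adds instances at equal distance steps, cycling through meshes or picking by seeded stream.
; Yaw is either random in snapped steps or a snapped offset that can follow the spline.
; Random scale and yaw ignore the seed, so they vary on each rebuild.
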(event EventBeginPlay)

(event Collision|EventActorBeginOverlap
  (params (OtherActor :type Actor%20Object%20Reference)))

(event EventTick
  (params (DeltaSeconds :type Float%20%28single-precision%29)))

(fn ConstructionScript
  (bind _meshes (Variables|Default|GetMeshes))
  (bind _min_uniform_scale_random (Variables|Randomize|GetMin%20Uniform%20Scale%20Random))
  (bind _max_uniform_scale_random (Variables|Randomize|GetMax%20Uniform%20Scale%20Random))
  (bind _total_number_of_meshes (Variables|Default|GetTotal%20Number%20of%20Meshes))
  (bind _yaw_rotation_ (Variables|Default|GetYaw%20Rotation%20))
  (bind _yaw_rotation_snap_degree (Variables|Default|GetYaw%20Rotation%20Snap%20Degree))
  (bind _hisms (Variables|Default|GetHISMs))
  (bind _uniform_scale (Variables|Default|GetUniform%20Scale))
  (bind _returnvalue (Utilities|Array|Length _hisms))
  (bind _returnvalue_2 (/ _yaw_rotation_ _yaw_rotation_snap_degree))
  (bind _returnvalue_3 (Math|Random|RandomFloatinRange _min_uniform_scale_random _max_uniform_scale_random))
  (bind _returnvalue_4 (* _uniform_scale _returnvalue_3))
  (bind _returnvalue_5 (* _returnvalue_2 _yaw_rotation_snap_degree))
  (bind _returnvalue_6 (Math|Conversions|ToFloat(Integer) _returnvalue_5))
  (for (_ _array_index) _meshes
    (Spline|SetClosedLoop (Variables|Default|GetSpline) (Variables|Default|GetClosed%20Spline) true)
    (bind _returnvalue_7 (AddComponent|AddHierarchicalInstancedStaticMeshComponent false))
    (Utilities|Array|Add (Variables|Default|GetHISMs) _returnvalue_7)
    (Components|StaticMesh|SetStaticMesh _returnvalue_7 (Utilities|Array|Get(acopy) _meshes _array_index))
    (Collision|SetCollisionEnabled _returnvalue_7 (Variables|Default|GetCollision%20Type)))
  (for _index (range 0 (- _total_number_of_meshes (Variables|Default|GetLast%20Index%20-%20Index%20Count)))
    (Components|InstancedStaticMesh|AddInstance (select (Variables|Randomize|GetRandom%20Placement%20Mesh%20From%20Array) (Utilities|Array|Get(acopy) _hisms (Class|KismetMathLibrary|RandomIntegerfromStream _returnvalue (Variables|Randomize|GetRandom%20Placement%20Seed))) (Utilities|Array|Get(acopy) _hisms (Math|Integer|%(Integer) _index _returnvalue))) (Math|Transform|MakeTransform (.Location (Math|Transform|BreakTransform (Spline|GetTransformatDistanceAlongSpline (Variables|Default|GetSpline) (* _index (/ (Spline|GetSplineLength (Variables|Default|GetSpline)) (Math|Conversions|ToFloat(Integer) _total_number_of_meshes))) "Local" false))) (Math|Rotator|SelectRotator (Math|Rotator|MakeRotator 0.0 0.0 (Math|Conversions|ToFloat(Integer) (* _yaw_rotation_snap_degree (Math|Random|RandomIntegerinRange 0 (/ (Variables|Randomize|GetMaxDegreeRandomRotation) _yaw_rotation_snap_degree))))) (Math|Rotator|MakeRotator (.Roll (Math|Rotator|BreakRotator (.Rotation (Math|Transform|BreakTransform (Spline|GetTransformatDistanceAlongSpline (Variables|Default|GetSpline) (* _index (/ (Spline|GetSplineLength (Variables|Default|GetSpline)) (Math|Conversions|ToFloat(Integer) _total_number_of_meshes))) "Local" false))))) (.Pitch (Math|Rotator|BreakRotator (.Rotation (Math|Transform|BreakTransform (Spline|GetTransformatDistanceAlongSpline (Variables|Default|GetSpline) (* _index (/ (Spline|GetSplineLength (Variables|Default|GetSpline)) (Math|Conversions|ToFloat(Integer) _total_number_of_meshes))) "Local" false))))) (Math|Float|SelectFloat (+ (.Yaw (Math|Rotator|BreakRotator (.Rotation (Math|Transform|BreakTransform (Spline|GetTransformatDistanceAlongSpline (Variables|Default|GetSpline) (* _index (/ (Spline|GetSplineLength (Variables|Default|GetSpline)) (Math|Conversions|ToFloat(Integer) _total_number_of_meshes))) "Local" false))))) _returnvalue_6) _returnvalue_6 (Variables|Default|GetOrient%20Meshes%20to%20Spline))) (Variables|Randomize|GetYaw%20Rotation%20Random)) (+ (Variables|Default|GetFree%20Scale%20) (Math|Vector|MakeVector _returnvalue_4 _returnvalue_4 _returnvalue_4))) false)))